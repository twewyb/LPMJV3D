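; BP_door_room11 is the door Blueprint for room 11, with a French text line telling the player to open the door to exit.
; While BP_ThirdPersonCharacter overlaps its trigger, it shows a widget and binds Spawn_caillou to the character's interact event, undoing both on exit.
; Despite that text, interacting only moves the referenced caillou (pebble) actor back to its spawn point; no door-opening logic appears here.
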(event `self.ReceiveBeginPlay`
  (set `self.line` "Pour sortir ouvre la porte"))

(event `self.trigger.OnComponentBeginOverlap`
  (params (OverlappedComponent :type "PrimitiveComponent Object Reference") (OtherActor :type "Actor Object Reference") (OtherComp :type "PrimitiveComponent Object Reference") (OtherBodyIndex :type Integer) (bFromSweep :type Boolean) (SweepResult :type "HitResult Structure (by ref)"))
  (bind _asbp_third_person_character (cast `/Game/ThirdPerson/Blueprints/BP_ThirdPersonCharacter` OtherActor))
  (add `/Game/ThirdPerson/Blueprints/BP_ThirdPersonCharacter.Interact` _asbp_third_person_character (delegate `Spawn_caillou`))
  (`SceneComponent.SetVisibility` (`self.Widget`) true false))

(event `self.trigger.OnComponentEndOverlap`
  (params (OverlappedComponent :type "PrimitiveComponent Object Reference") (OtherActor :type "Actor Object Reference") (OtherComp :type "PrimitiveComponent Object Reference") (OtherBodyIndex :type Integer))
  (bind _asbp_third_person_character (cast `/Game/ThirdPerson/Blueprints/BP_ThirdPersonCharacter` OtherActor))
  (remove `/Game/ThirdPerson/Blueprints/BP_ThirdPersonCharacter.Interact` _asbp_third_person_character (delegate `Spawn_caillou`))
  (`SceneComponent.SetVisibility` (`self.Widget`) false false))

(event `Spawn_caillou`
  (bind _caillou_reference (`self.Caillou_reference`))
  (`self.K2_SetActorTransform` _caillou_reference (`/Game/Blueprints/Renaud/BP_caillou_room1.Spawn point` _caillou_reference) false false))

(fn `UserConstructionScript`
  (`parent.UserConstructionScript`))