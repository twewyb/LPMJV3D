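; BP_Caillou_room1 is an interactable object, apparently a rock in room 1, that opens a referenced door.
; When the third-person character overlaps Box1, it binds OpenDoor to the character's interact event and shows a prompt widget; leaving the box reverses both.
; OpenDoor casts the door reference to BP_door_room11 and plays that door's ActorSequence.
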(event `self.Box1.OnComponentBeginOverlap`
  (params (OverlappedComponent :type "PrimitiveComponent Object Reference") (OtherActor :type "Actor Object Reference") (OtherComp :type "PrimitiveComponent Object Reference") (OtherBodyIndex :type Integer) (bFromSweep :type Boolean) (SweepResult :type "HitResult Structure (by ref)"))
  (bind _asbp_third_person_character (cast `/Game/ThirdPerson/Blueprints/BP_ThirdPersonCharacter` OtherActor))
  (add `/Game/ThirdPerson/Blueprints/BP_ThirdPersonCharacter.Interact` _asbp_third_person_character (delegate `OpenDoor`))
  (`SceneComponent.SetVisibility` (`self.Widget`) true false))

(event `self.Box1.OnComponentEndOverlap`
  (params (OverlappedComponent :type "PrimitiveComponent Object Reference") (OtherActor :type "Actor Object Reference") (OtherComp :type "PrimitiveComponent Object Reference") (OtherBodyIndex :type Integer))
  (bind _asbp_third_person_character (cast `/Game/ThirdPerson/Blueprints/BP_ThirdPersonCharacter` OtherActor))
  (remove `/Game/ThirdPerson/Blueprints/BP_ThirdPersonCharacter.Interact` _asbp_third_person_character (delegate `OpenDoor`))
  (`SceneComponent.SetVisibility` (`self.Widget`) false false))

(event `OpenDoor`
  (bind _asbp_door_room_11 (cast `/Game/Blueprints/BP_door_room11` (`self.DoorReference`)))
  (`ActorSequenceComponent.PlaySequence` (`/Game/Blueprints/BP_door_room11.ActorSequence` _asbp_door_room_11)))

(fn `UserConstructionScript`)