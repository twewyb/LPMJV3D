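; BP_NPC_room1 is an NPC Blueprint that offers an interaction prompt to the third-person player.
; Entering its trigger binds Interact to the player's interact event and shows a widget, unless HadTalk is set; leaving unbinds and hides it.
; Interacting hides the widget and sets SkipLine, then reaches a DoOnce with nothing after it.
; No dialogue logic appears in this graph, and HadTalk is only read here.
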(event `self.trigger.OnComponentBeginOverlap`
  (params (OverlappedComponent :type "PrimitiveComponent Object Reference") (OtherActor :type "Actor Object Reference") (OtherComp :type "PrimitiveComponent Object Reference") (OtherBodyIndex :type Integer) (bFromSweep :type Boolean) (SweepResult :type "HitResult Structure (by ref)"))
  (bind _asbp_third_person_character (cast `/Game/ThirdPerson/Blueprints/BP_ThirdPersonCharacter` OtherActor))
  (if (not (`self.hadTalk`))
    (add `/Game/ThirdPerson/Blueprints/BP_ThirdPersonCharacter.Interact` _asbp_third_person_character (delegate `Interact`))
    (`SceneComponent.SetVisibility` (`self.Widget`) true false)))

(event `Interact`
  (`SceneComponent.SetVisibility` (`self.Widget`) false false)
  (set `self.skipLine` true)
  (`/Engine/EditorBlueprintResources/StandardMacros.DoOnce` false))

(event `self.trigger.OnComponentEndOverlap`
  (params (OverlappedComponent :type "PrimitiveComponent Object Reference") (OtherActor :type "Actor Object Reference") (OtherComp :type "PrimitiveComponent Object Reference") (OtherBodyIndex :type Integer))
  (bind _asbp_third_person_character (cast `/Game/ThirdPerson/Blueprints/BP_ThirdPersonCharacter` OtherActor))
  (remove `/Game/ThirdPerson/Blueprints/BP_ThirdPersonCharacter.Interact` _asbp_third_person_character (delegate `Interact`))
  (`SceneComponent.SetVisibility` (`self.Widget`) false false))

(fn `UserConstructionScript`)