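; BP_Caillou_Ouvre is an interactable actor that lets the player open a linked door.
; When a BP_ThirdPersonCharacter begins overlapping it, it shows its widget and binds OpenDoor to that character's interact event.
; Ending the overlap hides the widget and removes the binding.
; OpenDoor plays the actor sequence on the referenced Door.
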(event `self.ReceiveActorBeginOverlap`
  (params (OtherActor :type "Actor Object Reference"))
  (bind _asbp_third_person_character (cast `/Game/ThirdPerson/Blueprints/BP_ThirdPersonCharacter` OtherActor))
  (add `/Game/ThirdPerson/Blueprints/BP_ThirdPersonCharacter.Interact` _asbp_third_person_character (delegate `OpenDoor`))
  (`SceneComponent.SetVisibility` (`self.Widget`) true false))

(event `self.ReceiveActorEndOverlap`
  (params (OtherActor :type "Actor Object Reference"))
  (bind _asbp_third_person_character (cast `/Game/ThirdPerson/Blueprints/BP_ThirdPersonCharacter` OtherActor))
  (remove `/Game/ThirdPerson/Blueprints/BP_ThirdPersonCharacter.Interact` _asbp_third_person_character (delegate `OpenDoor`))
  (`SceneComponent.SetVisibility` (`self.Widget`) false false))

(event `OpenDoor`
  (`ActorSequenceComponent.PlaySequence` (`/Game/Blueprints/BP_Fran/BP_Door_Fran.ActorSequence` (`self.door`))))

(fn `UserConstructionScript`)