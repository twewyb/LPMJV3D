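; BP_Door_Fran is an interactable rock door that blasts open when the player uses it.
; Overlapping Box1 shows a prompt widget and binds OpenDoor to the third-person character's interact event; leaving hides it and unbinds.
; OpenDoor spawns an explosion, hides the referenced big rock and disables its collision, then reveals every BP_Petit_Caillou with collision and unhides the referenced opened-rock actor.
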(event `self.Box1.OnComponentBeginOverlap`
  (params (OverlappedComponent :type "PrimitiveComponent Object Reference") (OtherActor :type "Actor Object Reference") (OtherComp :type "PrimitiveComponent Object Reference") (OtherBodyIndex :type Integer) (bFromSweep :type Boolean) (SweepResult :type "HitResult Structure (by ref)"))
  (bind _asbp_third_person_character (cast `/Game/ThirdPerson/Blueprints/BP_ThirdPersonCharacter` OtherActor))
  (add `/Game/ThirdPerson/Blueprints/BP_ThirdPersonCharacter.Interact` _asbp_third_person_character (delegate `OpenDoor`))
  (`SceneComponent.SetVisibility` (`self.Widget`) true false))

(event `self.Box1.OnComponentEndOverlap`
  (params (OverlappedComponent :type "PrimitiveComponent Object Reference") (OtherActor :type "Actor Object Reference") (OtherComp :type "PrimitiveComponent Object Reference") (OtherBodyIndex :type Integer))
  (bind _asbp_third_person_character (cast `/Game/ThirdPerson/Blueprints/BP_ThirdPersonCharacter` OtherActor))
  (remove `/Game/ThirdPerson/Blueprints/BP_ThirdPersonCharacter.Interact` _asbp_third_person_character (delegate `OpenDoor`))
  (`SceneComponent.SetVisibility` (`self.Widget`) false false))

(event `OpenDoor`
  (bind _grrrroscaillou (`self.GrrrrosCaillou`))
  (`GameplayStatics.SpawnEmitterAtLocation` "/Game/StarterContent/Particles/P_Explosion.P_Explosion" (+ (`self.K2_GetActorLocation`) (-50.0 0.0 125.0)))
  (`SceneComponent.SetVisibility` (`self.Widget`) false false)
  (`self.SetActorHiddenInGame` _grrrroscaillou true)
  (`PrimitiveComponent.SetCollisionEnabled` (`/Game/Blueprints/BP_Fran/BP_grosCaillouParle.rock` _grrrroscaillou) "NoCollision")
  (`|ExecutionSequence`
    (:`then_0`
      (bind _outactors (`GameplayStatics.GetAllActorsOfClass` "/Game/Blueprints/BP_Fran/BP_Petit_Caillou.BP_Petit_Caillou_C"))
      (for _array_element _outactors
        (bind _staticmesh (`/Game/Blueprints/BP_Fran/BP_Petit_Caillou.StaticMesh` _array_element))
        (`SceneComponent.SetVisibility` _staticmesh true false)
        (`PrimitiveComponent.SetCollisionEnabled` _staticmesh "QueryAndPhysics")))
    (:`then_1`
      (`GameplayStatics.GetAllActorsOfClass` "/Game/Blueprints/BP_Fran/BP_Caillou_Ouvre.BP_Caillou_Ouvre_C")
      (`self.SetActorHiddenInGame` (`self.caillououvre`) false))))

(fn `UserConstructionScript`)